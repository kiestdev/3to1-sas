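; BP_SpellFiring fires the demo spell when the player triggers the IA_Shoot input, provided firing is off cooldown and the player controller has enough mana.
; It spawns BP_DemoSpell at the player pawn's eye viewpoint, facing the view direction.
; It then deducts the mana cost from BP_FirstPersonPlayerController, found through GetActorOfClass, and uses a short Delay on the IsFireable flag as a cooldown.
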(event Input|EnhancedActionEvents|EnhancedInputActionIA_Shoot
  (params (ActionValue :type Boolean) (ElapsedSeconds :type Float%20%28double-precision%29) (TriggeredSeconds :type Float%20%28double-precision%29) (InputAction :type Input%20Action%20Object%20Reference :default "/Game/Input/Actions/IA_Shoot.IA_Shoot"))
  (bind _returnvalue (Game|Player|GetPlayerPawn 0))
  (bind (_outlocation _outrotation) (Actor|GetActorEyesViewPoint _returnvalue))
  ;[0.15 0.15 0.15 0.5] Demo Spell Firing
  (bind _returnvalue_2 (Actor|GetActorOfClass "/Game/FirstPerson/Blueprints/BP_FirstPersonPlayerController.BP_FirstPersonPlayerController_C"))
  (if (and (Variables|Default|GetIsFireable) (>= (Variables|/Game/FirstPerson/Blueprints/BP_FirstPersonPlayerController.BP_FirstPersonPlayerController_C|GetMana _returnvalue_2) 1e+02))
    (Variables|Default|SetIsFireable false)
    (Game|SpawnActorfromClass "/Game/Weapons/DemoSpell/BP_DemoSpell.BP_DemoSpell_C" (Math|Transform|MakeTransform _outlocation _outrotation "1.000000,1.000000,1.000000") "Undefined" "MultiplyWithRoot" 0 0)
    ;[0.15 0.15 0.15 0.5] Mana Spending And Spell Cooldown
    (bind _returnvalue_3 (Actor|GetActorOfClass "/Game/FirstPerson/Blueprints/BP_FirstPersonPlayerController.BP_FirstPersonPlayerController_C"))
    (Variables|/Game/FirstPerson/Blueprints/BP_FirstPersonPlayerController.BP_FirstPersonPlayerController_C|SetMana _returnvalue_3 (- (Variables|/Game/FirstPerson/Blueprints/BP_FirstPersonPlayerController.BP_FirstPersonPlayerController_C|GetMana _returnvalue_3) 1e+02))
    (Utilities|FlowControl|Delay 0.75)
    (Variables|Default|SetIsFireable true)))