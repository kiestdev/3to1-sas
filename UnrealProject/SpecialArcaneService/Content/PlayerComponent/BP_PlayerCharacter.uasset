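; BP_PlayerCharacter is a player character Blueprint with Enhanced Input handlers for mouse look, movement and running.
; IA_MouseLook calls Look, feeding its value only to UpDown, which drives controller yaw, while pitch receives zero.
; IA_Move calls Move, which applies input along actor forward and right vectors, but both scales are currently zero.
; IA_Run and the construction script are empty.
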(event Input|EnhancedActionEvents|EnhancedInputActionIA_Move
  (params (ActionValue :type Boolean) (ElapsedSeconds :type Float%20%28double-precision%29) (TriggeredSeconds :type Float%20%28double-precision%29) (InputAction :type Input%20Action%20Object%20Reference :default "/Game/PlayerComponent/Input/Actions/IA_Move.IA_Move"))
  (CallFunction|Move 0.0 0.0))

(event Input|EnhancedActionEvents|EnhancedInputActionIA_Run
  (params (ActionValue :type Boolean) (ElapsedSeconds :type Float%20%28double-precision%29) (TriggeredSeconds :type Float%20%28double-precision%29) (InputAction :type Input%20Action%20Object%20Reference :default "/Game/PlayerComponent/Input/Actions/IA_Run.IA_Run")))

(event Input|EnhancedActionEvents|EnhancedInputActionIA_MouseLook
  (params (ActionValue :type Float%20%28double-precision%29) (ElapsedSeconds :type Float%20%28double-precision%29) (TriggeredSeconds :type Float%20%28double-precision%29) (InputAction :type Input%20Action%20Object%20Reference :default "/Game/PlayerComponent/Input/Actions/IA_MouseLook.IA_MouseLook"))
  (CallFunction|Look ActionValue 0.0))

(fn ConstructionScript)

(fn Look
  (params (Up/Down :type Float%20%28single-precision%29) (Left/Right :type Float%20%28single-precision%29))
  (Pawn|Input|AddControllerYawInput Up/Down)
  (Pawn|Input|AddControllerPitchInput Left/Right))

(fn Move
  (params (Forward/Backward :type Float%20%28double-precision%29) (Right/Left :type Float%20%28single-precision%29))
  (Pawn|Input|AddMovementInput (Transformation|GetActorForwardVector) Forward/Backward false)
  (Pawn|Input|AddMovementInput (Transformation|GetActorRightVector) Right/Left false))